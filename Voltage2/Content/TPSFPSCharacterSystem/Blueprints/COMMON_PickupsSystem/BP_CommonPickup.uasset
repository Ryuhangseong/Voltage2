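; BP_CommonPickup is a common pickup actor that tracks whether the player is close enough to pick it up.
; Its Sphere's begin and end overlap events set and clear a CanPickup flag, only on authority and only for the pawn of player controller 0.
; GetCanPickup exposes the flag; the Blueprint itself holds no collection logic.
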(event OnComponentBeginOverlap(Sphere)
  (params (OverlappedComponent :type Primitive%20Component%20Object%20Reference) (OtherActor :type Actor%20Object%20Reference) (OtherComp :type Primitive%20Component%20Object%20Reference) (OtherBodyIndex :type Integer) (bFromSweep :type Boolean) (SweepResult :type Hit%20Result%20Structure%20%28by%20ref%29))
  ;[1 1 1] Overlaping Logic
  (if (== OtherActor (Pawn|GetControlledPawn (Game|GetPlayerController 0)))
    (Networking|SwitchHasAuthority
      (:Authority
        (Variables|Default|SetCan%20Pickup? true)))))

(event OnComponentEndOverlap(Sphere)
  (params (OverlappedComponent :type Primitive%20Component%20Object%20Reference) (OtherActor :type Actor%20Object%20Reference) (OtherComp :type Primitive%20Component%20Object%20Reference) (OtherBodyIndex :type Integer))
  ;[1 1 1] Overlaping Logic
  (if (== OtherActor (Pawn|GetControlledPawn (Game|GetPlayerController 0)))
    (Networking|SwitchHasAuthority
      (:Authority
        (Variables|Default|SetCan%20Pickup? false)))))

(event EventBeginPlay)

(event Collision|EventActorBeginOverlap
  (params (OtherActor :type Actor%20Object%20Reference)))

(event EventTick
  (params (DeltaSeconds :type Float%20%28single-precision%29)))

(fn ConstructionScript)

(fn GetCanPickup
  (return (Variables|Default|GetCan%20Pickup?)))