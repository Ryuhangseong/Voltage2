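; Base weapon actor for the TPS/FPS character system, holding basic weapon properties and current ammo state.
; On BeginPlay, the authority fills the ammo state from the clip size and ammo size in its basic properties.
; A multicast event plays a given sound at the weapon's location with a volume multiplier, and a getter exposes the swap time.
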(event Custom|MulticastPlayerWeaponSound
  (params (Sound :type Sound%20Base%20Object%20Reference) (VolumeMultiplier :type Float%20%28single-precision%29))
  ;[1 1 1] PLAY WEAPON SOUND
  (CallFunction|PlaySoundonWeapon Sound VolumeMultiplier))

(event Custom|InitializeWeaponProperties
  (bind _basic_weapon_properties (Variables|WEAPONSYSTEMPROPERTIES|GetBasic%20Weapon%20Properties))
  (bind (_firerate _clipsize _ammosize) (Utilities|Struct|BreakSTR_BasicWeaponProperties _basic_weapon_properties))
  ;[1 1 1] INITIALIZE
  ;;[1 1 1] Initialize
  ;;;[1 1 1] On swapn weapon
  (Variables|NOTEDIT|SetCurrent%20Ammo%20State (Utilities|Struct|MakeSTR_CurrentAmmoState _clipsize _ammosize)))

(event EventBeginPlay
  ;[1 1 1] EVENT BEGIN PLAY
  (Networking|SwitchHasAuthority
    (:Authority
      (CallFunction|InitializeWeaponProperties))))

(fn ConstructionScript)

(fn PlaySoundonWeapon
  (params (Sound :type Sound%20Base%20Object%20Reference) (VolumeMultiplier :type Float%20%28single-precision%29))
  (Audio|PlaySoundatLocation Sound (Transformation|GetActorLocation) "0, 0, 0" VolumeMultiplier 1.0 0.0 0 0 0))

(fn GetSwapTime
  (return (.SwapTime (Utilities|Struct|BreakSTR_BasicWeaponProperties (Variables|WEAPONSYSTEMPROPERTIES|GetBasic%20Weapon%20Properties)))))